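; BP_AudioCharacter is a character that drives a two-track music mixer through its AudioSystemActorComponent.
; On BeginPlay it adds an audio component, hands it to the system component as the mixer, activates it, and sets battle and jungle tracks with fade times and gains.
; Capsule begin and end overlap events are forwarded to the system component's owner overlap handlers.
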(event OnComponentBeginOverlap(CapsuleComponent)
  (params (OverlappedComponent :type Primitive%20Component%20Object%20Reference) (OtherActor :type Actor%20Object%20Reference) (OtherComp :type Primitive%20Component%20Object%20Reference) (OtherBodyIndex :type Integer) (bFromSweep :type Boolean) (SweepResult :type Hit%20Result%20Structure%20%28by%20ref%29))
  (Class|AudioSystemActorComponent|OnOwnerBeginOverlap (Variables|Default|GetAudioSystemActorComponent) OtherActor))

(event OnComponentEndOverlap(CapsuleComponent)
  (params (OverlappedComponent :type Primitive%20Component%20Object%20Reference) (OtherActor :type Actor%20Object%20Reference) (OtherComp :type Primitive%20Component%20Object%20Reference) (OtherBodyIndex :type Integer))
  (Class|AudioSystemActorComponent|OnOwnerEndOverlap (Variables|Default|GetAudioSystemActorComponent)))

(event EventBeginPlay
  (bind _audiosystemactorcomponent (Variables|Default|GetAudioSystemActorComponent))
  (bind _returnvalue (AddComponent|AddAudioComponent false))
  (Variables|/Script/DynamicAudioSystemCode.AudioSystemActorComponent|SetmMixer _audiosystemactorcomponent _returnvalue)
  (Class|AudioSystemActorComponent|ActivateMixer _audiosystemactorcomponent)
  (Class|AudioSystemActorComponent|SetAllParameters _audiosystemactorcomponent "/DynamicAudioSystemCode/Audio/battle_music_village_wav.battle_music_village_wav" "/DynamicAudioSystemCode/Audio/jungle_tribal_hut.jungle_tribal_hut" 1.5 1.5 1.0 1.0 1.0 1.0))

(fn ConstructionScript)