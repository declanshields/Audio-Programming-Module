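; BP_AreaTrigger is an area marker Blueprint that holds an AreaTrack object and a MajorArea flag.
; On BeginPlay it sets its TextRender to the object name of AreaTrack, labelling the area with its track.
; Two getter functions expose the track and the flag.
; It has no overlap logic of its own, as the overlap and tick events are empty.
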(event EventBeginPlay
  (Rendering|Components|TextRender|SetText (Variables|Default|GetTextRender) (Utilities|Text|ToText(String) (Utilities|GetObjectName (Variables|Default|GetArea%20Track)))))

(event Collision|EventActorBeginOverlap
  (params (OtherActor :type Actor%20Object%20Reference)))

(event EventTick
  (params (DeltaSeconds :type Float%20%28single-precision%29)))

(fn ConstructionScript)

(fn GetAreaTrack
  (return (Variables|Default|GetArea%20Track)))

(fn GetIsMajorArea
  (return (Variables|Default|GetMajor%20Area)))